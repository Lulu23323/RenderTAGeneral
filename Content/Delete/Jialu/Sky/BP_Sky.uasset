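; Sky actor that runs a day-night cycle with sun, moon, sky atmosphere, height fog, sky light and volumetric clouds.
; Tick advances a 24-hour Time value and wraps it, rotating sun and moon opposite in pitch and sampling curves by Time for lighting, scattering and fog.
; Construction creates dynamic cloud and light-function shadow materials, giving both the same coverage and wind settings.
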(event `self.ReceiveTick`
  (params (DeltaSeconds :type "Float (single-precision)"))
  (bind _output_get (set `self.Time` (+ (/ DeltaSeconds 0.5) (`self.Time`))))
  (if (>= _output_get 24.0)
    (set `self.Time` 0.0)
    (else
      (`self.UpdateComponents`))))

(fn `SetComponentReferences`
  (set `self.SunRef` (`self.Light_Sun`))
  (set `self.MoonRef` (`self.Light_Moon`))
  (set `self.SkyAtmosphereRef` (`self.SkyAtmosphere`))
  (set `self.HeightFogRef` (`self.ExponentialHeightFog`))
  (set `self.SkyLightRef` (`self.SkyLight`)))

(fn `UpdateCloudsProperties`
  (bind (_cloudwinddirection_r _cloudwinddirection_g) (break `LinearColor` (`self.CloudWindDirection`)))
  (`MaterialInstanceDynamic.SetScalarParameterValue` (`self.CloudMaterialInstance`) "Cloud Coverage" (`self.CloudCoverage`))
  (`MaterialInstanceDynamic.SetScalarParameterValue` (`self.CloudMaterialInstance`) "Wind Speed" (`self.CloudWindSpeed`))
  (`MaterialInstanceDynamic.SetVectorParameterValue` (`self.CloudMaterialInstance`) "Wind Direction" (make `LinearColor` _cloudwinddirection_r _cloudwinddirection_g 0.0 1.0)))

(fn `UpdateCloudsShadowsProperties`
  (bind (_cloudwinddirection_r _cloudwinddirection_g) (break `LinearColor` (`self.CloudWindDirection`)))
  (`MaterialInstanceDynamic.SetScalarParameterValue` (`self.CloudShadowsMaterialInstance`) "Cloud Coverage" (`self.CloudCoverage`))
  (`MaterialInstanceDynamic.SetScalarParameterValue` (`self.CloudShadowsMaterialInstance`) "Wind Speed" (`self.CloudWindSpeed`))
  (`MaterialInstanceDynamic.SetVectorParameterValue` (`self.CloudShadowsMaterialInstance`) "Wind Direction" (make `LinearColor` _cloudwinddirection_r _cloudwinddirection_g 0.0 1.0)))

(fn `UpdateComponents`
  (`|ExecutionSequence`
    (:`then_0`
      ;[1 1 1] Sun
      (`SceneComponent.K2_SetRelativeRotation` (`self.SunRef`) (`KismetMathLibrary.MakeRotator` 0.0 (`self.TimeInDegrees`) (`self.SunAngle`)) false false)
      (`LightComponent.SetIntensity` (`self.SunRef`) (`CurveFloat.GetFloatValue` (`self.Curve_Sun_Intensity`) (`self.Time`)))
      (`LightComponent.SetLightColor` (`self.SunRef`) (`CurveLinearColor.GetLinearColorValue` (`self.Curve_Sun_Color`) (`self.Time`)) true))
    (:`then_1`
      ;[1 1 1] Moon
      (`SceneComponent.K2_SetRelativeRotation` (`self.MoonRef`) (`KismetMathLibrary.MakeRotator` 0.0 (+ (`self.TimeInDegrees`) 180.0) (`self.MoonAngle`)) false false)
      (`LightComponent.SetIntensity` (`self.MoonRef`) (`CurveFloat.GetFloatValue` (`self.Curve_Moon_Intensity`) (`self.Time`))))
    (:`then_2`
      ;[1 1 1] Sky Atmosphere
      (`SkyAtmosphereComponent.SetRayleighScattering` (`self.SkyAtmosphereRef`) (`CurveLinearColor.GetLinearColorValue` (`self.Curve_RayleighScattering`) (`self.Time`))))
    (:`then_3`
      ;[1 1 1] Height Fog
      (`ExponentialHeightFogComponent.SetFogInscatteringColor` (`self.HeightFogRef`) (`CurveLinearColor.GetLinearColorValue` (`self.Curve_Fog_InscatteringColor`) (`self.Time`)))
      (`ExponentialHeightFogComponent.SetFogDensity` (`self.HeightFogRef`) (`CurveFloat.GetFloatValue` (`self.Curve_Fog_Density`) (`self.Time`))))
    (:`then_4`
      ;[1 1 1] Sky Light
      (`SkyLightComponent.SetIntensity` (`self.SkyLightRef`) (`CurveFloat.GetFloatValue` (`self.Curve_SkyLight_Intensity`) (`self.Time`)))
      (`SkyLightComponent.SetLightColor` (`self.SkyLightRef`) (`CurveLinearColor.GetLinearColorValue` (`self.Curve_SkyLight_Color`) (`self.Time`))))))

(fn `UserConstructionScript`
  (`|ExecutionSequence`
    (:`then_0`
      ;[1 1 1] Set variables for all the components in the blueprint
      (`self.SetComponentReferences`))
    (:`then_1`
      ;[1 1 1] Update all the components properties using curves values
      (`self.UpdateComponents`))
    (:`then_2`
      ;[1 1 1] Create a dynamic material instance for the clouds material and set it in the Volumetric Cloud component
      (bind _returnvalue (`KismetMaterialLibrary.CreateDynamicMaterialInstance` "/Game/Delete/Jialu/Sky/Clouds/MI_VolumetricClouds.MI_VolumetricClouds"))
      (bind _output_get (set `self.CloudMaterialInstance` _returnvalue))
      (`VolumetricCloudComponent.SetMaterial` (`self.VolumetricCloud`) _output_get)
      ;[1 1 1] Create a dynamic material instance for the clouds shadows material and set it in the Sun and Moon components
      (bind _returnvalue_2 (`KismetMaterialLibrary.CreateDynamicMaterialInstance` "/Game/Delete/Jialu/Sky/Clouds/MLF_Clouds_Shadows.MLF_Clouds_Shadows"))
      (set `self.CloudShadowsMaterialInstance` _returnvalue_2)
      (`LightComponent.SetLightFunctionMaterial` (`self.Light_Moon`) (`self.CloudShadowsMaterialInstance`))
      (`LightComponent.SetLightFunctionMaterial` (`self.Light_Sun`) (`self.CloudShadowsMaterialInstance`)))
    (:`then_3`
      ;[1 1 1] Update parameters in the clouds material
      (`self.UpdateCloudsProperties`)
      ;[1 1 1] Update parameters in the clouds shadows material
      (`self.UpdateCloudsShadowsProperties`))))